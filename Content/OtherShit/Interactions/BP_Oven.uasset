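; BP_Oven is an interactable oven in an item-based puzzle, which reveals a carved number clue from a frozen steak.
; On Interact it reads the first two flags of the first-person game mode's Inventory array.
; With the first flag set, one interaction sets the second flag as steak inserted, and later ones print the melted-steak numbers.
; Without it, the oven prints a joke about jumping in.
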(event `/Game/OtherShit/Interactions/BPI_Interactable.Interact`
  (bind _asbp_first_person_game_mode (cast `/Game/FirstPerson/Blueprints/BP_FirstPersonGameMode` (`GameplayStatics.GetGameMode`)))
  (set `self.GameMode` _asbp_first_person_game_mode)
  (if (`|GetArrayItem` (`/Game/FirstPerson/Blueprints/BP_FirstPersonGameMode.Inventory` (`self.GameMode`)))
    (if (`|GetArrayItem` (`/Game/FirstPerson/Blueprints/BP_FirstPersonGameMode.Inventory` (`self.GameMode`)) 1)
      (`KismetSystemLibrary.PrintString` "The frozen steak melted, revealing a few number carved into the sides")
      (`KismetSystemLibrary.PrintString` "1, 9, 3, 13, 12, 9")
      (else
        (`KismetSystemLibrary.PrintString` "put steak in there")
        (`KismetArrayLibrary.Array_Set` (`/Game/FirstPerson/Blueprints/BP_FirstPersonGameMode.Inventory` (`self.GameMode`)) 1 true)))
    (else
      (`KismetSystemLibrary.PrintString` "yea, you jumped in the fucking oven"))))

(fn `UserConstructionScript`)