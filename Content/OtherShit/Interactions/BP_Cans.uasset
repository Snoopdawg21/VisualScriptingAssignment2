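; BP_Cans is a numbered can used in a placement puzzle, tracking whether it is in its correct spot.
; On BeginPlay it caches a reference to BP_FirstPersonGameMode.
; The GetNum event compares a requested number to CanNum and sets InCorrectSpot, calling CheckPlates on the game mode only when they match.
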(event `/Game/OtherShit/Interactions/BPI_Cans.GetNum`
  (params (LookingForNum :type Integer))
  (if (== LookingForNum (`self.canNum`))
    (set `self.inCorrectSpot` true)
    (`/Game/FirstPerson/Blueprints/BP_FirstPersonGameMode.checkPlates` (`self.GameMode`))
    (else
      (set `self.inCorrectSpot` false))))

(event `self.ReceiveBeginPlay`
  (bind _asbp_first_person_game_mode (cast `/Game/FirstPerson/Blueprints/BP_FirstPersonGameMode` (`GameplayStatics.GetGameMode`)))
  (set `self.GameMode` _asbp_first_person_game_mode))

(fn `UserConstructionScript`)