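; BP_Cupboards is an interactable cupboard that lets the player find and view a letter.
; The first Interact marks it opened, caches BP_FirstPersonGameMode and shows discovery text through it.
; Later interactions toggle the letter: showing clears all widgets, adds an image preview and lengthens the GameMode timer, while toggling off only shortens that timer.
; A separate AttemptBox function adds a capsule UI widget and is not called here.
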(event `/Game/OtherShit/Interactions/BPI_Interactable.Interact`
  (bind _game_mode (`self.Game Mode`))
  (if (`self.openedCupboard`)
    (if (`self.letterToggle`)
      (set `self.letterToggle` false)
      (set `/Game/FirstPerson/Blueprints/BP_FirstPersonGameMode.timer` 3.0 _game_mode)
      (else
        (set `self.letterToggle` true)
        (set `/Game/FirstPerson/Blueprints/BP_FirstPersonGameMode.timer` 10.0 _game_mode)
        (`WidgetLayoutLibrary.RemoveAllWidgets`)
        (bind _returnvalue (`|CreateWidget` "/Game/OtherShit/UI_Elements/WBP_ImagePreviewUI.WBP_ImagePreviewUI_C"))
        (set `/Game/OtherShit/UI_Elements/WBP_ImagePreviewUI.image` "/Game/OtherShit/MyAssets/I_Letter.I_Letter" _returnvalue)
        (`UserWidget.AddToViewport` _returnvalue 0)))
    (else
      (set `self.openedCupboard` true)
      (bind _asbp_first_person_game_mode (cast `/Game/FirstPerson/Blueprints/BP_FirstPersonGameMode` (`GameplayStatics.GetGameMode`)))
      (bind _output_get (set `self.Game Mode` _asbp_first_person_game_mode))
      (`/Game/FirstPerson/Blueprints/BP_FirstPersonGameMode.ChangeText` _output_get "Looking through the cupboards, you find a sheet of paper"))))

(fn `AttemptBox`
  (locals (Capsule :type "Array of /Game/OtherShit/UI_Elements/WBP_CapsuleUI Object Reference"))
  (bind _returnvalue (`|CreateWidget` "/Game/OtherShit/UI_Elements/WBP_CapsuleUI.WBP_CapsuleUI_C"))
  (bind _output_get (set `self.UI` _returnvalue))
  (`UserWidget.AddToViewport` _output_get 0))

(fn `UserConstructionScript`)