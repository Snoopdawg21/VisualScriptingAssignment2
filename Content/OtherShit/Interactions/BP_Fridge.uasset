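; BP_Fridge is an interactable fridge that stays locked until a required inventory flag is set, then yields a frozen steak once.
; Interact reads boolean Inventory slots on BP_FirstPersonGameMode and reports locked, found or empty through its ChangeText.
; Finding the steak also shows an image preview widget and sets the steak's flag, along with a second ArraySet that has no explicit index.
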(event `/Game/OtherShit/Interactions/BPI_Interactable.Interact`
  (bind _game_mode (`self.Game Mode`))
  (bind _inventory (`/Game/FirstPerson/Blueprints/BP_FirstPersonGameMode.Inventory` (`self.Game Mode`)))
  (bind _asbp_first_person_game_mode (cast `/Game/FirstPerson/Blueprints/BP_FirstPersonGameMode` (`GameplayStatics.GetGameMode`)))
  (bind _output_get (set `self.Game Mode` _asbp_first_person_game_mode))
  (if (`|GetArrayItem` (`/Game/FirstPerson/Blueprints/BP_FirstPersonGameMode.Inventory` (`self.Game Mode`)) 2)
    (if (`|GetArrayItem` (`/Game/FirstPerson/Blueprints/BP_FirstPersonGameMode.Inventory` (`self.Game Mode`)) 3)
      (`/Game/FirstPerson/Blueprints/BP_FirstPersonGameMode.ChangeText` _game_mode "The rest of the fridge is empty.")
      (else
        (`/Game/FirstPerson/Blueprints/BP_FirstPersonGameMode.ChangeText` _game_mode "You found a frozen steak.")
        (bind _returnvalue (`|CreateWidget` "/Game/OtherShit/WBP_ImagePreviewUI.WBP_ImagePreviewUI_C"))
        (`UserWidget.AddToViewport` _returnvalue 0)
        (`KismetArrayLibrary.Array_Set` _inventory 0 true)
        (`KismetArrayLibrary.Array_Set` _inventory 3 true)))
    (else
      (`/Game/FirstPerson/Blueprints/BP_FirstPersonGameMode.ChangeText` _output_get "The Fridge is Locked!"))))

(fn `UserConstructionScript`)