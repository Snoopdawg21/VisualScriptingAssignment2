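; BP_Exit is an interactable exit door with a code-entry prompt.
; Its Interact event alternates: first it shows a six-letter code hint through the first-person game mode, then it clears all widgets, opens WBP_ExitUI and sets the game mode's Timer.
; A separate OpeningDoor event plays the LiftDoor timeline, lerping the actor's world Z between fixed heights to raise it.
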(event `self.ReceiveBeginPlay`
  (bind _asbp_first_person_game_mode (cast `/Game/FirstPerson/Blueprints/BP_FirstPersonGameMode` (`GameplayStatics.GetGameMode`)))
  (set `self.Game Mode` _asbp_first_person_game_mode))

(event `/Game/OtherShit/Interactions/BPI_Interactable.Interact`
  (if (`self.interacted`)
    (`WidgetLayoutLibrary.RemoveAllWidgets`)
    (bind _returnvalue (`|CreateWidget` "/Game/OtherShit/UI_Elements/WBP_ExitUI.WBP_ExitUI_C"))
    (`UserWidget.AddToViewport` _returnvalue 0)
    (set `self.interacted` false)
    (set `/Game/FirstPerson/Blueprints/BP_FirstPersonGameMode.timer` 10.0 (`self.Game Mode`))
    (else
      (bind _asbp_first_person_game_mode (cast `/Game/FirstPerson/Blueprints/BP_FirstPersonGameMode` (`GameplayStatics.GetGameMode`)))
      (`/Game/FirstPerson/Blueprints/BP_FirstPersonGameMode.ChangeText` _asbp_first_person_game_mode "Next to the door you can input a code. It takes 6 letters.")
      (set `self.interacted` true))))

(event `OpeningDoor`
  (bind (_returnvalue_x _returnvalue_y) (`KismetMathLibrary.BreakVector` (`self.K2_GetActorLocation`)))
  (bind (_direction _lift_it) (`Timeline|LiftDoor`)
    (:`Update`
      (`self.K2_SetActorLocation` (`KismetMathLibrary.MakeVector` _returnvalue_x _returnvalue_y (`KismetMathLibrary.Lerp` 200.0 620.0 _lift_it))))))

(fn `UserConstructionScript`)